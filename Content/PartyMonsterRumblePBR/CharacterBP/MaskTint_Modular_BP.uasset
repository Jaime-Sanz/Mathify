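; Modular mask-tint character Blueprint for the Party Monster Rumble PBR content, assembled from separate mesh parts.
; Gloves, body and head parts, eyes, mouths, noses and tails all follow the main skeletal mesh through Set Master Pose Component, so they share its pose.
; The link is made in both the Construction Script and BeginPlay; the graphs contain no tint or gameplay logic.
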(event `self.ReceiveBeginPlay`
  (`SkinnedMeshComponent.SetLeaderPoseComponent` (`self.Gloves`) (`self.SkeletalMeshComponent`) false)
  (`SkinnedMeshComponent.SetLeaderPoseComponent` (`self.Bodyparts`) (`self.SkeletalMeshComponent`) false)
  (`SkinnedMeshComponent.SetLeaderPoseComponent` (`self.Eyes`) (`self.SkeletalMeshComponent`) false)
  (`SkinnedMeshComponent.SetLeaderPoseComponent` (`self.Mouths`) (`self.SkeletalMeshComponent`) false)
  (`SkinnedMeshComponent.SetLeaderPoseComponent` (`self.Noses`) (`self.SkeletalMeshComponent`) false)
  (`SkinnedMeshComponent.SetLeaderPoseComponent` (`self.Tails`) (`self.SkeletalMeshComponent`) false)
  (`SkinnedMeshComponent.SetLeaderPoseComponent` (`self.Headparts`) (`self.SkeletalMeshComponent`) false))

(fn `UserConstructionScript`
  (`SkinnedMeshComponent.SetLeaderPoseComponent` (`self.Tails`) (`self.SkeletalMeshComponent`) false)
  (`SkinnedMeshComponent.SetLeaderPoseComponent` (`self.Noses`) (`self.SkeletalMeshComponent`) false)
  (`SkinnedMeshComponent.SetLeaderPoseComponent` (`self.Eyes`) (`self.SkeletalMeshComponent`) false)
  (`SkinnedMeshComponent.SetLeaderPoseComponent` (`self.Mouths`) (`self.SkeletalMeshComponent`) false)
  (`SkinnedMeshComponent.SetLeaderPoseComponent` (`self.Bodyparts`) (`self.SkeletalMeshComponent`) false)
  (`SkinnedMeshComponent.SetLeaderPoseComponent` (`self.Headparts`) (`self.SkeletalMeshComponent`) false)
  (`SkinnedMeshComponent.SetLeaderPoseComponent` (`self.Gloves`) (`self.SkeletalMeshComponent`) false))